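; Base 2D flipbook enemy that either patrols or turns its sprite to face the player.
; Player entry into ScreenZone starts a looping AI MoveTo between two target points.
; Player exit stops, hides and teleports it to spawn, and Tick reveals living patrollers once the player is outside the zone.
; DamageCollision can damage the player, while KillCollision kills the enemy, shifting it along Y and switching to a non-looping death flipbook.
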(event OnComponentBeginOverlap(ScreenZone)
  (params (OverlappedComponent :type Primitive%20Component%20Object%20Reference) (OtherActor :type Actor%20Object%20Reference) (OtherComp :type Primitive%20Component%20Object%20Reference) (OtherBodyIndex :type Integer) (bFromSweep :type Boolean) (SweepResult :type Hit%20Result%20Structure%20%28by%20ref%29))
  ;[1 1 1] Player detection to active behavior
  (Utilities|Casting|CastToBP_PlayerCharacter OtherActor)
  (if (not (Variables|Default|GetRespawning))
    (if (Variables|Default|GetPatrolBehavior)
      (if (not (Variables|Default|GetIsPatrolOn))
        (CallFunction|Patrol)))))

(event OnComponentEndOverlap(ScreenZone)
  (params (OverlappedComponent :type Primitive%20Component%20Object%20Reference) (OtherActor :type Actor%20Object%20Reference) (OtherComp :type Primitive%20Component%20Object%20Reference) (OtherBodyIndex :type Integer))
  ;[1 1 1] Player detection to active behavior
  (Utilities|Casting|CastToBP_PlayerCharacter OtherActor)
  (Utilities|FlowControl|Sequence
    (:then_0
      (Variables|Default|SetIsPatrolOn false))
    (:then_1
      (Variables|Default|SetRespawning true))
    (:then_2
      (Class|NavMovementComponent|StopActiveMovement (Variables|Character|GetCharacterMovement))
      (Rendering|SetVisibility (Variables|Default|GetSprite) false false)
      (Transformation|Teleport (Variables|Default|GetSpawnLocation) (Variables|Default|GetSpawnRotation)))))

(event OnComponentBeginOverlap(DamageCollision)
  (params (OverlappedComponent :type Primitive%20Component%20Object%20Reference) (OtherActor :type Actor%20Object%20Reference) (OtherComp :type Primitive%20Component%20Object%20Reference) (OtherBodyIndex :type Integer) (bFromSweep :type Boolean) (SweepResult :type Hit%20Result%20Structure%20%28by%20ref%29))
  ;[1 1 1] DamageCollision Behavior
  (bind _asbp_player_character (Utilities|Casting|CastToBP_PlayerCharacter OtherActor))
  (switch Utilities|FlowControl|Switch|SwitchonEDamageBehaviour (Variables|Default|GetDamageCollisionBehavior)
    (:NewEnumerator0
      (Default|OnDamage _asbp_player_character))))

(event OnComponentBeginOverlap(KillCollision)
  (params (OverlappedComponent :type Primitive%20Component%20Object%20Reference) (OtherActor :type Actor%20Object%20Reference) (OtherComp :type Primitive%20Component%20Object%20Reference) (OtherBodyIndex :type Integer) (bFromSweep :type Boolean) (SweepResult :type Hit%20Result%20Structure%20%28by%20ref%29))
  ;[1 1 1] Dead Behavior
  (Utilities|Casting|CastToBP_PlayerCharacter OtherActor)
  (|DeadGraph))

(event Custom|Patrol
  ;[1 1 1] Patrol
  (|PatrolGraph))

(event EventBeginPlay
  ;[1 1 1] Save Spawn location and rotation to re-spawn if need
  (Variables|Default|SetSpawnLocation (Transformation|GetActorLocation))
  (Variables|Default|SetSpawnRotation (Transformation|GetActorRotation)))

(event EventTick
  (params (DeltaSeconds :type Float%20%28single-precision%29))
  ;[1 1 1] Use tick to respawn if player not in the screen
  (if (not (Variables|Default|GetIsDead))
    (if (Variables|Default|GetPatrolBehavior)
      (|PatroTickSpawn)
      (else
        (|FollowPlayerGraph)))))

(fn ConstructionScript)

(event Custom|MovePatrol
  ;[1 1 1] Patrol movement
  (if (not (Variables|Default|GetIsDead))
    (if (Variables|Default|GetIsPatrolOn)
      (bind _asaicontroller (Utilities|Casting|CastToAIController (Pawn|GetController)))
      (AI|AIMoveTo _asaicontroller "0, 0, 0" (Variables|Default|GetStart%20Target%20Point) -1.0 "Default" "Default" false true
        (:OnMoveFinished
          (if (Variables|Default|GetIsPatrolOn)
            (if (not (Variables|Default|GetIsDead))
              (AI|AIMoveTo _asaicontroller "0, 0, 0" (Variables|Default|GetEnd%20Target%20Point) -1.0 "Default" "Default" false true
                (:OnMoveFinished
                  (CallFunction|MovePatrol))))))))))