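; BP_Rat is a rat enemy Blueprint whose own graph handles movement audio.
; Each tick it calls OnTickValidations, then plays its Audio component if X velocity is non-zero and the sound is neither playing nor on cooldown.
; A DelayAudio flag with a one-second Delay spaces out the replays.
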(event Collision|EventActorBeginOverlap
  (params (OtherActor :type Actor%20Object%20Reference)))

(event EventTick
  (params (DeltaSeconds :type Float%20%28single-precision%29))
  ;[1 1 1] Audio Behavior | Only on movement
  (Class|DKEnemy|OnTickValidations)
  (if (!= (.x (Transformation|GetVelocity)) 0.0)
    (if (not (or (Audio|Components|Audio|IsPlaying (Variables|Default|GetAudio)) (Variables|Default|GetDelayAudio)))
      (Variables|Default|SetDelayAudio true)
      (Audio|Components|Audio|Play (Variables|Default|GetAudio) 0.0)
      (Utilities|FlowControl|Delay 1.0)
      (Variables|Default|SetDelayAudio false))))

(fn ConstructionScript)