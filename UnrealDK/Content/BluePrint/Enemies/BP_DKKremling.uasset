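; Kremling enemy Blueprint that visually turns its 2D sprite to follow the player.
; The OnCharacteronScreen event passes an angle to FollowingPlayer, which picks the display from its absolute value in ten-degree bands.
; Both extremes show the right or left idle flipbook, while intermediate bands swap static turn frames on FollowPositionSprite, toggling visibility between the two components.
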(event EventBeginPlay
  (|CallParentFunction))

(event Collision|EventActorBeginOverlap
  (params (OtherActor :type Actor%20Object%20Reference)))

(event EventTick
  (params (DeltaSeconds :type Float%20%28single-precision%29))
  (|CallParentFunction DeltaSeconds) ; This node is disabled and will not be called.\nDrag off pins to build functionality.
)

(event EventOnCharacteronScreen
  (params (Angle :type Float%20%28single-precision%29))
  (CallFunction|FollowingPlayer Angle))

(fn ConstructionScript
  (|CallParentFunction))

(fn FollowingPlayer
  (params (A :type Float%20%28double-precision%29))
  (bind _followpositionsprite (Variables|Default|GetFollowPositionSprite))
  (bind _sprite (Variables|Default|GetSprite))
  (bind _sprite_2 (Variables|Default|GetSprite))
  (Variables|Default|SetAngleDirection (Math|Float|Absolute(Float) A))
  (Transformation|SetWorldRotation (Variables|Default|GetSprite) "0, 0, 0" false false)
  (if (< (Variables|Default|GetAngleDirection) 1e+01)
    (Rendering|SetVisibility _followpositionsprite false false)
    (Rendering|SetVisibility _sprite_2 true false)
    (Sprite|SetFlipbook _sprite_2 "/Game/Assets/Sprites/Enemies/dk_kremling_idle_right.dk_kremling_idle_right")
    (elif (< (Variables|Default|GetAngleDirection) 2e+01)
      (Variables|Default|SetCurrentSprite "/Game/Assets/Sprites/Enemies/SplitSprite/kremling/dk/with_coin/moving/kremlings_dk_kremling_15.kremlings_dk_kremling_15")
      (Rendering|Components|Sprite|SetSprite _followpositionsprite (Variables|Default|GetCurrentSprite) :!label _label)
      (Rendering|SetVisibility _followpositionsprite true false)
      (Rendering|SetVisibility _sprite_2 false false)
      (elif (< (Variables|Default|GetAngleDirection) 3e+01)
        (Variables|Default|SetCurrentSprite "/Game/Assets/Sprites/Enemies/SplitSprite/kremling/dk/with_coin/moving/kremlings_dk_kremling_14.kremlings_dk_kremling_14")
        (goto _label)
        (elif (< (Variables|Default|GetAngleDirection) 4e+01)
          (Variables|Default|SetCurrentSprite "/Game/Assets/Sprites/Enemies/SplitSprite/kremling/dk/with_coin/moving/kremlings_dk_kremling_13.kremlings_dk_kremling_13")
          (goto _label)
          (elif (< (Variables|Default|GetAngleDirection) 5e+01)
            (Variables|Default|SetCurrentSprite "/Game/Assets/Sprites/Enemies/SplitSprite/kremling/dk/with_coin/moving/kremlings_dk_kremling_12.kremlings_dk_kremling_12")
            (goto _label)
            (elif (< (Variables|Default|GetAngleDirection) 6e+01)
              (Variables|Default|SetCurrentSprite "/Game/Assets/Sprites/Enemies/SplitSprite/kremling/dk/with_coin/moving/kremlings_dk_kremling_11.kremlings_dk_kremling_11")
              (goto _label)
              (elif (< (Variables|Default|GetAngleDirection) 7e+01)
                (Variables|Default|SetCurrentSprite "/Game/Assets/Sprites/Enemies/SplitSprite/kremling/dk/with_coin/moving/kremlings_dk_kremling_10.kremlings_dk_kremling_10")
                (goto _label)
                (elif (< (Variables|Default|GetAngleDirection) 8e+01)
                  (Variables|Default|SetCurrentSprite "/Game/Assets/Sprites/Enemies/SplitSprite/kremling/dk/with_coin/moving/kremlings_dk_kremling_9.kremlings_dk_kremling_9")
                  (goto _label)
                  (elif (< (Variables|Default|GetAngleDirection) 9e+01)
                    (Variables|Default|SetCurrentSprite "/Game/Assets/Sprites/Enemies/SplitSprite/kremling/dk/with_coin/moving/kremlings_dk_kremling_8.kremlings_dk_kremling_8")
                    (goto _label)
                    (elif (< (Variables|Default|GetAngleDirection) 1e+02)
                      (Variables|Default|SetCurrentSprite "/Game/Assets/Sprites/Enemies/SplitSprite/kremling/dk/with_coin/moving/kremlings_dk_kremling_7.kremlings_dk_kremling_7")
                      (goto _label)
                      (elif (< (Variables|Default|GetAngleDirection) 1.1e+02)
                        (Variables|Default|SetCurrentSprite "/Game/Assets/Sprites/Enemies/SplitSprite/kremling/dk/with_coin/moving/kremlings_dk_kremling_6.kremlings_dk_kremling_6")
                        (goto _label)
                        (elif (< (Variables|Default|GetAngleDirection) 1.2e+02)
                          (Variables|Default|SetCurrentSprite "/Game/Assets/Sprites/Enemies/SplitSprite/kremling/dk/with_coin/moving/kremlings_dk_kremling_5.kremlings_dk_kremling_5")
                          (goto _label)
                          (elif (< (Variables|Default|GetAngleDirection) 1.3e+02)
                            (Variables|Default|SetCurrentSprite "/Game/Assets/Sprites/Enemies/SplitSprite/kremling/dk/with_coin/moving/kremlings_dk_kremling_4.kremlings_dk_kremling_4")
                            (goto _label)
                            (elif (< (Variables|Default|GetAngleDirection) 1.4e+02)
                              (Variables|Default|SetCurrentSprite "/Game/Assets/Sprites/Enemies/SplitSprite/kremling/dk/with_coin/moving/kremlings_dk_kremling_3.kremlings_dk_kremling_3")
                              (goto _label)
                              (elif (< (Variables|Default|GetAngleDirection) 1.5e+02)
                                (Variables|Default|SetCurrentSprite "/Game/Assets/Sprites/Enemies/SplitSprite/kremling/dk/with_coin/moving/kremlings_dk_kremling_2.kremlings_dk_kremling_2")
                                (goto _label)
                                (elif (< (Variables|Default|GetAngleDirection) 1.6e+02)
                                  (Variables|Default|SetCurrentSprite "/Game/Assets/Sprites/Enemies/SplitSprite/kremling/dk/with_coin/moving/kremlings_dk_kremling_1.kremlings_dk_kremling_1")
                                  (goto _label)
                                  (elif (< (Variables|Default|GetAngleDirection) 1.7e+02)
                                    (Variables|Default|SetCurrentSprite "/Game/Assets/Sprites/Enemies/SplitSprite/kremling/dk/with_coin/moving/kremlings_dk_kremling_0.kremlings_dk_kremling_0")
                                    (goto _label)
                                    (else
                                      (Rendering|SetVisibility (Variables|Default|GetFollowPositionSprite) false false)
                                      (Rendering|SetVisibility _sprite true false)
                                      (Sprite|SetFlipbook _sprite "/Game/Assets/Sprites/Enemies/dk_kremling_idle_left.dk_kremling_idle_left"))))))))))))))))))))