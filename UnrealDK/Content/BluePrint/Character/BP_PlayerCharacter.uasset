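; BP_PlayerCharacter is a sprite-based player character with movement, run and jump input, animated through an AnimInstance state machine.
; Movement input flips the sprite by direction, run input switches walk speed, and jump either jumps or adds upward movement when swimming.
; Jump, ledge and landing events trigger animation jump nodes, and entering or leaving water plays a splash.
; Damage and kill events only print debug text, and rope-climbing logic is disconnected.
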(event Custom|OnKillEnemy
  (Development|PrintString "Jump!"))

(event Custom|OnDamage
  (Development|PrintString "I need to be dead!"))

(event Input|EnhancedActionEvents|EnhancedInputActionIA_Movement
  (params (ActionValue :type Float%20%28double-precision%29) (ElapsedSeconds :type Float%20%28double-precision%29) (TriggeredSeconds :type Float%20%28double-precision%29) (InputAction :type Input%20Action%20Object%20Reference :default "/Game/BluePrint/Character/IA_Movement.IA_Movement"))
  (bind _sprite (Variables|Default|GetSprite))
  ;[1 1 1] Movement
  (:Triggered
    (Pawn|Input|AddMovementInput (Transformation|GetActorForwardVector) ActionValue false)
    (if (> ActionValue 0.0)
      (Transformation|SetWorldRotation _sprite "0, 0, 0" false false)
      (else
        (Transformation|SetWorldRotation _sprite "0.000000,-180.000000,0.000000" false false)))))

(event Input|EnhancedActionEvents|EnhancedInputActionIA_Run
  (params (ActionValue :type Boolean) (ElapsedSeconds :type Float%20%28double-precision%29) (TriggeredSeconds :type Float%20%28double-precision%29) (InputAction :type Input%20Action%20Object%20Reference :default "/Game/BluePrint/Character/IA_Run.IA_Run"))
  (bind _charactermovement (Variables|Character|GetCharacterMovement))
  ;[1 1 1] IA Toggle Run
  (:Triggered
    (Variables|/Script/Engine.CharacterMovementComponent|SetMaxWalkSpeed _charactermovement 3e+02)
    (Variables|Default|SetisRunning true))
  (:Started
    (Variables|Default|SetisAttack ActionValue :!label _label)
    (Variables|/Script/Engine.CharacterMovementComponent|SetMaxWalkSpeed _charactermovement 1.2e+02)
    (Variables|Default|SetisRunning false))
  (:Completed
    (goto _label)))

(event Input|EnhancedActionEvents|EnhancedInputActionIA_Jump
  (params (ActionValue :type Boolean) (ElapsedSeconds :type Float%20%28double-precision%29) (TriggeredSeconds :type Float%20%28double-precision%29) (InputAction :type Input%20Action%20Object%20Reference :default "/Game/BluePrint/Character/IA_Jump.IA_Jump"))
  (bind _returnvalue (Transformation|GetActorForwardVector))
  ;[1 1 1] IA Jump
  (:Triggered
    (switch Utilities|FlowControl|Switch|SwitchonEMovementMode (Variables|/Script/Engine.CharacterMovementComponent|GetMovementMode (Variables|Character|GetCharacterMovement))
      (:MOVE_Walking
        (Character|Jump))
      (:MOVE_Swimming
        (Pawn|Input|AddMovementInput (Math|Vector|MakeVector (.x _returnvalue) (.y _returnvalue) 1.0) 1.0 false)
        (Development|PrintString "on the watter")
        (Development|PrintString (Utilities|String|ToString(Float) (.z _returnvalue)))))))

(event EventBeginPlay)

(event EventOnMovementModeChanged
  (params (PrevMovementMode :type EMovementMode%20Enum :default "MOVE_None") (NewMovementMode :type EMovementMode%20Enum :default "MOVE_None") (PrevCustomMode :type Byte :default 0) (NewCustomMode :type Byte :default 0))
  ;[0.4438 0.1079 0.4896] OnChangeMovementMode || Use in swimming to change sound
  (if (or (Utilities|Enum|Equal(Enum) NewMovementMode "MOVE_Swimming") (Utilities|Enum|Equal(Enum) PrevMovementMode "MOVE_Swimming"))
    (Audio|PlaySound2D "/Game/Assets/Audio/SFX/Environment/Splash_Swamp_Cue.Splash_Swamp_Cue" 1.0 1.0 0.0 0 0)))

(event EventTick
  (params (DeltaSeconds :type Float%20%28single-precision%29)))

(event EventOnJumped
  ;[1 1 1] IA Jump
  (Class|PaperZDAnimInstance|JumptoNode (Variables|/Script/PaperZD.PaperZDAnimationComponent|GetAnimInstance (Variables|Default|GetAnimationComponent)) "Airborne" "None"))

(event EventOnWalkingOffLedge
  (params (PreviousFloorImpactNormal :type Vector%20%28by%20ref%29 :default "0, 0, 0") (PreviousFloorContactNormal :type Vector%20%28by%20ref%29 :default "0, 0, 0") (PreviousLocation :type Vector%20%28by%20ref%29 :default "0, 0, 0") (TimeDelta :type Float%20%28single-precision%29))
  ;[1 1 1] IA Jump
  (Class|PaperZDAnimInstance|JumptoNode (Variables|/Script/PaperZD.PaperZDAnimationComponent|GetAnimInstance (Variables|Default|GetAnimationComponent)) "Airborne" "None"))

(event EventOnLanded
  (params (Hit :type Hit%20Result%20Structure%20%28by%20ref%29))
  ;[1 1 1] IA Jump
  (Class|PaperZDAnimInstance|JumptoNode (Variables|/Script/PaperZD.PaperZDAnimationComponent|GetAnimInstance (Variables|Default|GetAnimationComponent)) "Landed" "None"))

(fn ConstructionScript)