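; BP_Dixie is the playable Dixie Kong Paper2D character, with Enhanced Input movement, jumping and flipbook animation.
; Move input drives walk/idle flipbooks and flips sprite rotation by direction unless jumping.
; Jump plays a one-shot flipbook, then a Delay loop polls vertical velocity until zero to restore idle.
; Tick gates a fall flipbook on IsStartFalling, which this graph only ever clears.
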(event Input|EnhancedActionEvents|EnhancedInputActionIA_Movement
  (params (ActionValue :type Float%20%28double-precision%29) (ElapsedSeconds :type Float%20%28double-precision%29) (TriggeredSeconds :type Float%20%28double-precision%29) (InputAction :type Input%20Action%20Object%20Reference :default "/Game/BluePrint/Character/IA_Movement.IA_Movement"))
  (bind _sprite (Variables|Default|GetSprite))
  ;[1 1 1] IA_Move | AnimationChange
  (:Triggered
    (Pawn|Input|AddMovementInput (Transformation|GetActorForwardVector) ActionValue false)
    (if (not (Variables|Default|GetIsJumping))
      (Sprite|SetFlipbook (Variables|Default|GetSprite) "/Game/Assets/Character/DixieKong/DixieKong_walking.DixieKong_walking")
      (if (> ActionValue 0.0)
        (Transformation|SetWorldRotation _sprite "0, 0, 0" false false)
        (else
          (Transformation|SetWorldRotation _sprite "0.000000,-180.000000,0.000000" false false)))))
  (:Completed
    (if (not (Variables|Default|GetIsJumping))
      (Sprite|SetFlipbook (Variables|Default|GetSprite) "/Game/Assets/Character/DixieKong/DixieKong_dixie_idle.DixieKong_dixie_idle"))))

(event Input|EnhancedActionEvents|EnhancedInputActionIA_Jump
  (params (ActionValue :type Boolean) (ElapsedSeconds :type Float%20%28double-precision%29) (TriggeredSeconds :type Float%20%28double-precision%29) (InputAction :type Input%20Action%20Object%20Reference :default "/Game/BluePrint/Character/IA_Jump.IA_Jump"))
  (bind _sprite (Variables|Default|GetSprite))
  ;[1 1 1] IA_Jump | Animaction Change
  (:Triggered
    (if (not (Variables|Default|GetIsJumping))
      (Variables|Default|SetIsJumping true)
      (Character|Jump)
      (Components|Timeline|SetLooping _sprite false)
      (Sprite|SetFlipbook _sprite "/Game/Assets/Character/DixieKong/Dixie_jump.Dixie_jump")
      (Utilities|FlowControl|Delay 0.1)
      (if (== (.Z (Math|Vector|BreakVector (Transformation|GetVelocity))) 0.0) :!label _label
        (Components|Timeline|SetLooping _sprite true)
        (Audio|Components|Audio|Play _sprite)
        (Sprite|SetFlipbook _sprite "/Game/Assets/Character/DixieKong/DixieKong_dixie_idle.DixieKong_dixie_idle")
        (Variables|Default|SetIsJumping false)
        (else
          (Utilities|FlowControl|Delay 0.2)
          (goto _label))))))

(event EventBeginPlay
  ;[1 1 1] IMC Default
  (bind _asbp_player_controller (Utilities|Casting|CastToBP_PlayerController (Pawn|GetController)))
  (Input|AddMappingContext (PlayerController|LocalPlayerSubsystems|GetEnhancedInputLocalPlayerSubsystem _asbp_player_controller) "/Game/BluePrint/Character/IMC_Default.IMC_Default" 0 "(bIgnoreAllPressedKeysUntilRelease=True,bForceImmediately=False)"))

(event EventTick
  (params (DeltaSeconds :type Float%20%28single-precision%29))
  (bind _sprite (Variables|Default|GetSprite))
  (if (< (.Z (Math|Vector|BreakVector (Transformation|GetVelocity))) 0.0)
    (if (Variables|Default|GetisStartFalling)
      (Components|Timeline|SetLooping _sprite false)
      (Sprite|SetFlipbook _sprite "/Game/Assets/Character/DixieKong/Dixie_Fall.Dixie_Fall")
      (Variables|Default|SetisStartFalling false))
    (else
      (Variables|Default|SetisStartFalling false))))

(fn ConstructionScript)