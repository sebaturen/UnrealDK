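; BP_Dixie is the player-controlled Dixie Kong character, a flipbook sprite that walks and jumps.
; On BeginPlay it adds IMC_Default to the player controller's Enhanced Input subsystem.
; Movement input moves it along the actor forward vector, plays the walking flipbook and rotates only the sprite to face the input sign, returning to idle on release.
; Jump input calls Jump and switches to the Barrel_save flipbook, with no landing logic.
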(event Input|EnhancedActionEvents|EnhancedInputActionIA_Movement
  (params (ActionValue :type Float%20%28double-precision%29) (ElapsedSeconds :type Float%20%28double-precision%29) (TriggeredSeconds :type Float%20%28double-precision%29) (InputAction :type Input%20Action%20Object%20Reference :default "/Game/BluePrint/IA_Movement.IA_Movement"))
  (bind _sprite (Variables|Default|GetSprite))
  ;[1 1 1] IA_Move | AnimationChange
  (:Triggered
    (Pawn|Input|AddMovementInput (Transformation|GetActorForwardVector) ActionValue false)
    (Sprite|SetFlipbook (Variables|Default|GetSprite) "/Game/Assets/Character/DixieKong/DixieKong_walking.DixieKong_walking")
    (if (> ActionValue 0.0)
      (Transformation|SetWorldRotation _sprite "0, 0, 0" false false)
      (else
        (Transformation|SetWorldRotation _sprite "0.000000,-180.000000,0.000000" false false))))
  (:Completed
    (Sprite|SetFlipbook (Variables|Default|GetSprite) "/Game/Assets/Character/DixieKong/DixieKong_dixie_idle.DixieKong_dixie_idle")))

(event Input|EnhancedActionEvents|EnhancedInputActionIA_Jump
  (params (ActionValue :type Boolean) (ElapsedSeconds :type Float%20%28double-precision%29) (TriggeredSeconds :type Float%20%28double-precision%29) (InputAction :type Input%20Action%20Object%20Reference :default "/Game/BluePrint/IA_Jump.IA_Jump"))
  (:Triggered
    (Character|Jump)
    (Sprite|SetFlipbook (Variables|Default|GetSprite) "/Game/Assets/ObjectsAndEffects/barrel_save.barrel_save")))

(event EventBeginPlay
  ;[1 1 1] IMC Default
  (bind _asbp_player_controller (Utilities|Casting|CastToBP_PlayerController (Pawn|GetController)))
  (Input|AddMappingContext (PlayerController|LocalPlayerSubsystems|GetEnhancedInputLocalPlayerSubsystem _asbp_player_controller) "/Game/BluePrint/IMC_Default.IMC_Default" 0 "(bIgnoreAllPressedKeysUntilRelease=True,bForceImmediately=False)"))

(fn ConstructionScript)