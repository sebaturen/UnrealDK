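; BPA_Barrel is a 2D barrel actor with four variants: Save Point, DK, Bonus and W.
; The Construction Script switches on TypeBox to set the appearance.
; Save Point and DK swap the PaperFlipbook animation, while Bonus and W hide it and show BarrelBonus with their own sprite.
; It holds no gameplay logic, as its event graph contains only disabled placeholder events.
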(event EventBeginPlay)

(event Collision|EventActorBeginOverlap
  (params (OtherActor :type Actor%20Object%20Reference)))

(event EventTick
  (params (DeltaSeconds :type Float%20%28single-precision%29)))

(fn ConstructionScript
  (bind _paperflipbook (Variables|Default|GetPaperFlipbook))
  (switch Utilities|FlowControl|Switch|SwitchonBarrelTyps (Variables|Default|GetTypeBox)
    (:NewEnumerator0
      (Sprite|SetFlipbook _paperflipbook "/Game/Assets/Sprites/ObjectsAndEffects/barrel_save.barrel_save"))
    (:NewEnumerator1
      (Sprite|SetFlipbook _paperflipbook "/Game/Assets/Sprites/ObjectsAndEffects/barrel_dk.barrel_dk"))
    (:NewEnumerator2
      (Rendering|SetVisibility (Variables|Default|GetBonusSprite) true false)
      (Rendering|SetVisibility (Variables|Default|GetBarrelBonus) true false :!label _label)
      (Rendering|SetVisibility (Variables|Default|GetPaperFlipbook) false false))
    (:NewEnumerator3
      (Rendering|SetVisibility (Variables|Default|GetWSprite) true false)
      (goto _label))))