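; Banana bunch collectible actor with a Paper2D flipbook and a box collider, collected through its PickUp event.
; PickUp plays a 2D sound, calls PickUpAnimation, disables the box's collision and starts a fast looping timer.
; The timer fires SwapVisiblity, which flips a boolean to blink the sprite.
; Overlap handling and removal of the actor are not in these graphs.
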(event Custom|SwapVisiblity
  (Rendering|SetVisibility (Variables|Default|GetPaperFlipbook) (Variables|Default|GetSwapVisibility) false)
  (Variables|Default|SetSwapVisibility (not (Variables|Default|GetSwapVisibility))))

(event EventBeginPlay)

(event Collision|EventActorBeginOverlap
  (params (OtherActor :type Actor%20Object%20Reference)))

(event EventTick
  (params (DeltaSeconds :type Float%20%28single-precision%29)))

(event EventPickUp
  (Audio|PlaySound2D "/Game/Assets/Audio/SFX/Items/Banana_bunch_DKC3_Cue.Banana_bunch_DKC3_Cue" 1.0 1.0 0.0 0 0)
  (Class|BananaBunch|PickUpAnimation)
  (Collision|SetCollisionEnabled (Variables|Default|GetBox) "NoCollision")
  (Utilities|Time|SetTimerbyEvent (delegate Custom|SwapVisiblity) 0.2 true))

(fn ConstructionScript)